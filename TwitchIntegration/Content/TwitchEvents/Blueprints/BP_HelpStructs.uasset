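; Help platform actor in the TwitchEvents folder that appears temporarily when SpawnHelp is called, and starts hidden with collision off.
; SpawnHelp shows it with collision, then after a five-second delay hides it again unless something stands on it.
; Box overlaps track occupancy with an unfiltered flag; if occupied at timeout, removal is deferred until the next end overlap.
; Removal only hides the actor and disables collision, so it is reusable.
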(event OnComponentBeginOverlap(Box)
  (params (OverlappedComponent :type Primitive%20Component%20Object%20Reference) (OtherActor :type Actor%20Object%20Reference) (OtherComp :type Primitive%20Component%20Object%20Reference) (OtherBodyIndex :type Integer) (bFromSweep :type Boolean) (SweepResult :type Hit%20Result%20Structure%20%28by%20ref%29))
  ;[1 1 1] Set variable when actor stands on platform
  (Variables|Default|SetStandingOn true))

(event OnComponentEndOverlap(Box)
  (params (OverlappedComponent :type Primitive%20Component%20Object%20Reference) (OtherActor :type Actor%20Object%20Reference) (OtherComp :type Primitive%20Component%20Object%20Reference) (OtherBodyIndex :type Integer))
  ;[1 1 1] Set variable when actor leaves platform
  (Variables|Default|SetStandingOn false)
  (if (Variables|Default|GetDeleteWhenLeave)
    (Variables|Default|SetDeleteWhenLeave false)
    (Rendering|SetActorHiddenInGame true)
    (Collision|SetActorEnableCollision false)))

(event Custom|SpawnHelp
  (Rendering|SetActorHiddenInGame false)
  (Collision|SetActorEnableCollision true)
  (Utilities|FlowControl|Delay 5.0)
  (if (Variables|Default|GetStandingOn)
    (Variables|Default|SetDeleteWhenLeave true)
    (else
      (Rendering|SetActorHiddenInGame true)
      (Collision|SetActorEnableCollision false))))

(event EventBeginPlay
  ;[1 1 1] Hide help on start
  (Rendering|SetActorHiddenInGame true)
  (Collision|SetActorEnableCollision false))

(fn ConstructionScript)