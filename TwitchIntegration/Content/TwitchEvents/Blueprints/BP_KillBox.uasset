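; BP_KillBox is a kill volume that, on any actor overlap, teleports the BP_ThirdPersonCharacter to the selected saved spawn point, keeping its rotation.
; SetSpawn appends the character's location to SpawnList when it is grounded and increments ArrayPointer, which selects the respawn location.
; LastSpawn and NextSpawn step that pointer back or forward through the saved points, stopping at either end of the list.
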(event Custom|SetSpawn
  (bind _returnvalue (Actor|GetActorOfClass "/Game/ThirdPerson/Blueprints/BP_ThirdPersonCharacter.BP_ThirdPersonCharacter_C"))
  (bind _grounded (Default|CheckGrounded _returnvalue))
  (if _grounded
    (bind _returnvalue_2 (Actor|GetActorOfClass "/Game/ThirdPerson/Blueprints/BP_ThirdPersonCharacter.BP_ThirdPersonCharacter_C"))
    (Utilities|Array|Add (Variables|Default|GetSpawnList) (Transformation|GetActorLocation _returnvalue_2))
    (Variables|Default|SetArrayPointer (+ (Variables|Default|GetArrayPointer) 1))))

(event Custom|LastSpawn
  (if (not (== (- (Variables|Default|GetArrayPointer) 1) -1))
    (Variables|Default|SetArrayPointer (- (Variables|Default|GetArrayPointer) 1))))

(event Custom|NextSpawn
  (if (not (== (+ (Variables|Default|GetArrayPointer) 1) (Utilities|Array|Length (Variables|Default|GetSpawnList))))
    (Variables|Default|SetArrayPointer (+ (Variables|Default|GetArrayPointer) 1))))

(event Collision|EventActorBeginOverlap
  (params (OtherActor :type Actor%20Object%20Reference))
  (bind _returnvalue (Actor|GetActorOfClass "/Game/ThirdPerson/Blueprints/BP_ThirdPersonCharacter.BP_ThirdPersonCharacter_C"))
  (Transformation|Teleport _returnvalue (Utilities|Array|Get(acopy) (Variables|Default|GetSpawnList) (Variables|Default|GetArrayPointer)) (Transformation|GetActorRotation _returnvalue)))

(fn ConstructionScript)