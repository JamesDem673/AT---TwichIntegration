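; StaticBox is a cube Blueprint in the TwitchEvents folder whose colour can be switched between blue, red and green.
; The construction script creates a dynamic material instance on the Cube and applies the stored Colour to its "Colour" vector parameter.
; Three custom events each overwrite Colour with a fixed value and push it to that material instance; nothing in this file calls them.
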(event Custom|Change%20Colour%20Green
  (bind _output_get (Variables|Default|SetColour "(R=0.010000,G=1.000000,B=0.000000,A=1.000000)"))
  (Rendering|Material|SetVectorParameterValue (Variables|Default|GetDynamicMat) "Colour" _output_get :!class /Script/Engine.MaterialInstanceDynamic))

(event Custom|Change%20Colour%20Blue
  (bind _output_get (Variables|Default|SetColour "(R=0.000000,G=0.000000,B=1.000000,A=1.000000)"))
  (Rendering|Material|SetVectorParameterValue (Variables|Default|GetDynamicMat) "Colour" _output_get :!class /Script/Engine.MaterialInstanceDynamic))

(event Custom|Change%20Colour%20Red
  (bind _output_get (Variables|Default|SetColour "(R=1.000000,G=0.000000,B=0.000000,A=1.000000)"))
  (Rendering|Material|SetVectorParameterValue (Variables|Default|GetDynamicMat) "Colour" _output_get :!class /Script/Engine.MaterialInstanceDynamic))

(fn ConstructionScript
  (bind _returnvalue (Rendering|Material|CreateDynamicMaterialInstance (Variables|Default|GetCube) 0 0 "None" :!class /Script/Engine.PrimitiveComponent))
  (bind _output_get (Variables|Default|SetDynamicMat _returnvalue))
  (Rendering|Material|SetVectorParameterValue _output_get "Colour" (Variables|Default|GetColour) :!class /Script/Engine.MaterialInstanceDynamic))